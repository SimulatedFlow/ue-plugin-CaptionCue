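; Demo director actor for the CaptionCue subtitle and caption system that drives scripted and automatic dialogue.
; On BeginPlay it refreshes caption styles, gathers speaker actors and can open a mouse-driven control panel.
; With auto dialogue enabled, a looping timer cycles round-robin through the speakers, triggering each one's next line.
; PlayDialogueScene, not called within this Blueprint, issues a fixed exchange mixing named-speaker subtitles with speakerless captions.
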(event EventBeginPlay
  (bind _returnvalue (Game|GetPlayerController 0))
  (bind _returnvalue_2 (Subsystems|GetCaptionCueSubsystem))
  (Class|CaptionCueSubsystem|RefreshStyles _returnvalue_2)
  (Class|CaptionCueSubsystem|SetShowStats _returnvalue_2 (Variables|CaptionCueDemo|GetbShowStats))
  (bind _outactors (Actor|GetAllActorsOfClass "/CaptionCue/CaptionCue/Blueprints/BP_CaptionCueSpeaker.BP_CaptionCueSpeaker_C"))
  (Variables|Default|SetSpeakerActors _outactors)
  (if (Variables|CaptionCueDemo|GetbShowControlPanel)
    (bind _returnvalue_3 (UserInterface|CreateWidget "/CaptionCue/CaptionCue/UI/WBP_CaptionCueDemoPanel.WBP_CaptionCueDemoPanel_C" _returnvalue))
    (Variables|Default|SetControlPanel _returnvalue_3)
    (UserInterface|Viewport|AddtoViewport _returnvalue_3 0)
    (Input|SetInputModeGameandUI _returnvalue 0 "DoNotLock" false false)
    (Variables|/Script/Engine.PlayerController|SetbShowMouseCursor _returnvalue true))
  (if (Variables|CaptionCueDemo|GetbAutoDialogue)
    (Utilities|Time|SetTimerbyFunctionName self "DialogueStep" (Variables|CaptionCueDemo|GetDialogueIntervalSeconds) true)))

(event Collision|EventActorBeginOverlap
  (params (OtherActor :type Actor%20Object%20Reference)))

(event EventTick
  (params (DeltaSeconds :type Float%20%28single-precision%29)))

(fn ConstructionScript)

(fn PlayDialogueScene
  (Class|CaptionCueStatics|ShowSubtitle (Utilities|Text|MakeLiteralText "You hear that? Something moved behind the shutters.") "Mara")
  (Class|CaptionCueStatics|ShowSubtitle (Utilities|Text|MakeLiteralText "That building has been empty for nine years. Nothing moves in there.") "Detrick")
  (Class|CaptionCueStatics|ShowCaptionfromRequest (Utilities|Struct|MakeCaptionCueRequest (Utilities|Text|MakeLiteralText "low strings swell") "None" "" "Music"))
  (Class|CaptionCueStatics|ShowSubtitle (Utilities|Text|MakeLiteralText "Nine years is a long time for nothing to move.") "Mara")
  (Class|CaptionCueStatics|ShowCaptionfromRequest (Utilities|Struct|MakeCaptionCueRequest (Utilities|Text|MakeLiteralText "Objective updated: investigate the shutters") "None" "" "System" 0.0 10)))

(fn DialogueStep
  (bind _speakeractors (Variables|Default|GetSpeakerActors))
  (bind _returnvalue (Utilities|Array|Length _speakeractors))
  (if (> _returnvalue (Class|KismetSystemLibrary|MakeLiteralInteger))
    (Variables|Default|SetSpeakerCursor (+ (Math|Integer|%(Integer) (Variables|Default|GetSpeakerCursor) _returnvalue) (Class|KismetSystemLibrary|MakeLiteralInteger 1)))
    (bind _asbp_caption_cue_speaker (Utilities|Casting|CastToBP_CaptionCueSpeaker (Utilities|Array|Get(acopy) _speakeractors (Math|Integer|%(Integer) (Variables|Default|GetSpeakerCursor) _returnvalue))))
    (Default|SayNextLine _asbp_caption_cue_speaker)))