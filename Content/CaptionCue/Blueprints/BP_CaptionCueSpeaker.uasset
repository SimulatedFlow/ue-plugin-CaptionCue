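; BP_CaptionCueSpeaker is a speaker actor that shows its dialogue lines as subtitles, one per call.
; The construction script writes the display name to its NameTag.
; SayNextLine, if any lines exist, registers the speaker's ID, name and color, then shows the current line under that ID.
; It advances LineIndex with a modulo so the lines cycle, and the event graph holds no active logic.
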(event EventBeginPlay)

(event Collision|EventActorBeginOverlap
  (params (OtherActor :type Actor%20Object%20Reference)))

(event EventTick
  (params (DeltaSeconds :type Float%20%28single-precision%29)))

(fn ConstructionScript
  (Rendering|Components|TextRender|SetText (Variables|Default|GetNameTag) (Variables|CaptionCueDemo|GetDisplayName)))

(fn SayNextLine
  (bind _lines (Variables|CaptionCueDemo|GetLines))
  (bind _returnvalue (Utilities|Array|Length _lines))
  (if (> _returnvalue (Class|KismetSystemLibrary|MakeLiteralInteger))
    (Class|CaptionCueStatics|RegisterSpeaker (Variables|CaptionCueDemo|GetSpeakerId) (Variables|CaptionCueDemo|GetDisplayName) (Variables|CaptionCueDemo|GetSpeakerColor))
    (Class|CaptionCueStatics|ShowSubtitle (Utilities|Array|Get(acopy) _lines (Math|Integer|%(Integer) (Variables|Default|GetLineIndex) _returnvalue)) (Variables|CaptionCueDemo|GetSpeakerId))
    (Variables|Default|SetLineIndex (+ (Math|Integer|%(Integer) (Variables|Default|GetLineIndex) _returnvalue) (Class|KismetSystemLibrary|MakeLiteralInteger 1)))))